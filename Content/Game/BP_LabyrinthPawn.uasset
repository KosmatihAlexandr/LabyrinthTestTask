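; Player pawn for a labyrinth ball game that rotates either the camera or the referenced Labyrinth and shows a controls-hint widget on BeginPlay.
; Held mode inputs set RotationType through a SwitchRotationMode macro, which routes yaw and pitch axes to the pawn or, negated, to the Labyrinth.
; Other actions regenerate the Labyrinth or have it spawn a ball at the visibility trace hit under the cursor.
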(event `InputAxis|InputRotationYaw`
  (params (AxisValue :type "Float (single-precision)"))
  (switch `/Game/Game/InputRotationType` (`self.RotationType`)
    (:`NewEnumerator1`
      (`self.AddYaw` AxisValue))
    (:`NewEnumerator2`
      (bind _labyrinth (`self.Labyrinth`)
        (:`then`
          (`Labyrinth.AddYaw` _labyrinth (* AxisValue -1.0)))
        (:`else`)))))

(event `InputAxis|InputRotationPitch`
  (params (AxisValue :type "Float (single-precision)"))
  (switch `/Game/Game/InputRotationType` (`self.RotationType`)
    (:`NewEnumerator1`
      (`self.AddPitch` AxisValue))
    (:`NewEnumerator2`
      (bind _labyrinth (`self.Labyrinth`)
        (:`then`
          (`Labyrinth.AddPitch` _labyrinth (* AxisValue -1.0)))
        (:`else`)))))

(event `InputAction|CameraRotationMode`
  (params (Key :type "Key Structure"))
  (:`Pressed`
    (`self.SwitchRotationMode` "NewEnumerator1" :!label _label))
  (:`Released`
    (goto _label :!via `Released`)))

(event `InputAction|LabyrinthRotationMode`
  (params (Key :type "Key Structure"))
  (:`Pressed`
    (`self.SwitchRotationMode` "NewEnumerator2" :!label _label_2))
  (:`Released`
    (goto _label_2 :!via `Released`)))

(event `InputAction|RebuildLabyrinth`
  (params (Key :type "Key Structure"))
  (:`Pressed`
    (bind _labyrinth (`self.Labyrinth`)
      (:`then`
        (`Labyrinth.GenerateLabyrinth` _labyrinth))
      (:`else`))))

(event `InputAction|AddBall`
  (params (Key :type "Key Structure"))
  (bind (_hitresult _returnvalue) (`PlayerController.GetHitResultUnderCursorByChannel` (`GameplayStatics.GetPlayerController` 0) "TraceTypeQuery1" false))
  (:`Pressed`
    (bind _labyrinth (`self.Labyrinth`)
      (:`then`
        (if _returnvalue
          (`Labyrinth.SpawnBall` _labyrinth (`.Location` (`GameplayStatics.BreakHitResult` _hitresult)))))
      (:`else`))))

(event `self.ReceiveBeginPlay`
  (`parent.ReceiveBeginPlay`)
  (bind _returnvalue (`|CreateWidget` "/Game/Game/Widget_ControlsHint.Widget_ControlsHint_C"))
  (`UserWidget.AddToViewport` _returnvalue 0))

(fn `UserConstructionScript`)